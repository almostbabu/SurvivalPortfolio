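; BP_DamageActor is a debug damage zone that hurts the first player character while it stands inside a box collider.
; Box overlap events set and clear an IsInside flag for that character and send DamageInstance through a damage interface message on entry.
; Tick resends the message while the flag is set, relying on a class-default tick interval, noted as two seconds, for pacing instead of a timer.
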(event `self.ReceiveTick`
  (params (DeltaSeconds :type "Float (single-precision)"))
  ;[1 1 1] Deal damage to player every 2 seconds (Check Class Defaults)
  (if (`self.IsInside?`)
    (message `/Game/SurvivalGame/Core/Character/Interfaces/INT_StatusEffects.Damage_Interface` (`GameplayStatics.GetPlayerCharacter` 0) (`self.DamageInstance`))))

(event `self.Box.OnComponentBeginOverlap`
  (params (OverlappedComponent :type "PrimitiveComponent Object Reference") (OtherActor :type "Actor Object Reference") (OtherComp :type "PrimitiveComponent Object Reference") (OtherBodyIndex :type Integer) (bFromSweep :type Boolean) (SweepResult :type "HitResult Structure (by ref)"))
  (bind _returnvalue (`GameplayStatics.GetPlayerCharacter` 0))
  ;[1 1 1] Checking if the player is inside the collider
  (if (== OtherActor _returnvalue)
    (set `self.IsInside?` true)
    (message `/Game/SurvivalGame/Core/Character/Interfaces/INT_StatusEffects.Damage_Interface` _returnvalue (`self.DamageInstance`))))

(event `self.Box.OnComponentEndOverlap`
  (params (OverlappedComponent :type "PrimitiveComponent Object Reference") (OtherActor :type "Actor Object Reference") (OtherComp :type "PrimitiveComponent Object Reference") (OtherBodyIndex :type Integer))
  ;[1 1 1] Checking if the player is inside the collider
  (if (== OtherActor (`GameplayStatics.GetPlayerCharacter` 0))
    (set `self.IsInside?` false)))

(fn `UserConstructionScript`)